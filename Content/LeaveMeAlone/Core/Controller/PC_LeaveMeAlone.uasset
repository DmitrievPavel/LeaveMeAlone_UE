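; Player controller for LeaveMeAlone that handles the pause menu and the death screen.
; The Pause input, guarded by an OnPause flag, stops the pawn's weapon fire, pauses the game and shows WBP_Pause with UI-only input and a visible cursor.
; UnPossess waits three seconds, then pauses the game and shows WBP_Dead the same way.
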(event EventBeginPlay)

(event EventTick
  (params (DeltaSeconds :type Float%20%28single-precision%29)))

(event EventUnPossess
  (params (UnpossessedPawn :type Pawn%20Object%20Reference))
  (Utilities|FlowControl|Delay 3.0)
  (Game|SetGamePaused true)
  (bind _returnvalue (UserInterface|CreateWidget "/Game/LeaveMeAlone/Widgets/UI/WBP_Dead.WBP_Dead_C"))
  (UserInterface|Viewport|AddtoViewport _returnvalue 0)
  (Input|SetInputModeUIOnly self 0 "DoNotLock" false)
  (Variables|Default|SetbShowMouseCursor true))

(event Input|ActionEvents|InputActionPause
  (params (Key :type Key%20Structure :default "None"))
  (:Pressed
    (if (not (Variables|Default|GetOnPause))
      (Variables|Default|SetOnPause true)
      (Class|LMAWeaponComponent|StopFire (Actor|GetComponentbyClass (Game|Player|GetPlayerPawn 0) "/Script/LeaveMeAlone.LMAWeaponComponent"))
      (Game|SetGamePaused true)
      (bind _returnvalue (UserInterface|CreateWidget "/Game/LeaveMeAlone/Widgets/UI/WBP_Pause.WBP_Pause_C"))
      (bind _output_get (Variables|Default|SetPauseWidget _returnvalue))
      (UserInterface|Viewport|AddtoViewport _output_get 0)
      (Input|SetInputModeUIOnly self _returnvalue "DoNotLock" false)
      (Variables|Default|SetbShowMouseCursor true))))

(fn ConstructionScript)