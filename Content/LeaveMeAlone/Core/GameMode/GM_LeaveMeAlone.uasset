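; Game mode for LeaveMeAlone that runs the match countdown and ends the game when time runs out.
; A looping one-second timer started on BeginPlay decrements GameTime and clears itself at zero.
; If the player character's health component does not report it dead at that point, the game pauses and shows WBP_GameOver with UI-only input and a visible cursor.
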(event Custom|CustomEvent
  (bind _output_get (Variables|Default|SetGameTime (- (Variables|Default|GetGameTime) 1)))
  (if (== _output_get 0)
    (Utilities|Time|ClearandInvalidateTimerbyHandle (Variables|Default|GetGameTimerHandle))
    (bind _aslmadefault_character (Utilities|Casting|CastToLMADefaultCharacter (Game|Player|GetPlayerPawn 0)))
    (if (not (Class|LMAHealthComponent|IsDead (Actor|GetComponentbyClass _aslmadefault_character "/Script/LeaveMeAlone.LMAHealthComponent")))
      (Game|SetGamePaused true)
      (bind _returnvalue (UserInterface|CreateWidget "/Game/LeaveMeAlone/Widgets/UI/WBP_GameOver.WBP_GameOver_C"))
      (UserInterface|Viewport|AddtoViewport _returnvalue 0)
      (bind _aspc_leave_me_alone (Utilities|Casting|CastToPC_LeaveMeAlone (Game|GetPlayerController 0)))
      (Input|SetInputModeUIOnly _aspc_leave_me_alone _returnvalue "DoNotLock" false)
      (Variables|/Script/Engine.PlayerController|SetbShowMouseCursor _aspc_leave_me_alone true))))

(event EventBeginPlay
  (bind _returnvalue (Utilities|Time|SetTimerbyEvent (delegate Custom|CustomEvent) 1.0 true))
  (Variables|Default|SetGameTimerHandle _returnvalue))

(event EventTick
  (params (DeltaSeconds :type Float%20%28single-precision%29)))

(fn ConstructionScript)